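; Ryokan lantern actor for the Japanese-style room that carries a configurable point light.
; The construction script copies exposed variables onto the PointLight: intensity, color temperature, shadow and volumetric shadow casting, mobility, volumetric scattering and attenuation radius.
; The event graph holds only disabled placeholder events, so the lantern has no runtime logic.
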(fn `UserConstructionScript`
  (bind _pointlight (`self.PointLight`))
  (`LightComponent.SetIntensity` _pointlight (`KismetMathLibrary.Conv_IntToDouble` (`self.LightIntensity`)))
  (`LightComponent.SetTemperature` _pointlight (`KismetMathLibrary.Conv_IntToDouble` (`self.Color Temperature`)))
  (`LightComponentBase.SetCastVolumetricShadow` _pointlight (`self.Cast VolumetricShadow`))
  (`LightComponentBase.SetCastShadows` _pointlight (`self.Cast Shadow`))
  (`SceneComponent.SetMobility` _pointlight (`self.Mobility`))
  (`LightComponent.SetVolumetricScatteringIntensity` _pointlight (`self.Vulumetric Scattering Intensity`))
  (`LocalLightComponent.SetAttenuationRadius` _pointlight (`self.AttenuationRad`)))