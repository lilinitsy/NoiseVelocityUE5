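; BP_Stones_01 is a construction-script Blueprint that lays stone meshes along an editable spline.
; It divides the spline length by DistanceBetweenStones and places a mesh at each step in local space.
; A random stream gives each stone a random yaw and a slightly varied uniform scale.
; Each stone gets its own new instanced static mesh component, rather than sharing one; the event graph is unused.
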(fn `UserConstructionScript`
  (bind _spline (`self.Spline`))
  (bind _distancebetweenstones (`self.DistanceBetweenStones`))
  (for _index (range (+ (`.ReturnValue` (`KismetMathLibrary.FMod` (`SplineComponent.GetSplineLength` _spline) _distancebetweenstones)) 1))
    (bind _returnvalue (`AddComponent|NODE_AddInstancedStaticMeshComponent-1`))
    (`StaticMeshComponent.SetStaticMesh` _returnvalue (`self.S_Mesh`))
    (`InstancedStaticMeshComponent.AddInstance` _returnvalue (`KismetMathLibrary.MakeTransform` (`SplineComponent.GetLocationAtDistanceAlongSpline` _spline (* _index _distancebetweenstones) "Local") (`KismetMathLibrary.MakeRotator` 0.0 0.0 (`KismetMathLibrary.RandomFloatInRangeFromStream` (`self.NewVar_1`) 0.0 360.0)) (`KismetMathLibrary.Conv_DoubleToVector` (`KismetMathLibrary.RandomFloatInRangeFromStream` (`self.NewVar_1`) 0.6 0.85))) false)))